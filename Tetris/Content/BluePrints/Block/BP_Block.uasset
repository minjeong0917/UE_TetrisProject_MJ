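; Falling Tetris piece that builds one of seven colored four-cube shapes at random in its construction script and starts at TetrisBoard height.
; Input moves it left, right or down in grid steps, repeating on timers while held; rotation is an empty stub.
; A looping DropBlock timer only traces below each cube; on a hit, it replaces the cubes with colored BP_SingleBlocks, spawns the next BP_Block and destroys itself.
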(event Custom|Right
  ;[0.15 0.15 0.15 0.5] Right Move
  (if (Variables|Default|GetIsDPush)
    (Transformation|AddActorWorldOffset "0.000000,-50.000000,0.000000")))

(event Custom|DropBlock
  (Variables|Default|SetIsDrop true)
  (for _array_element (Components|GetChildrenComponents (Variables|Default|GetDefaultSceneRoot) false)
    (bind _returnvalue (Collision|LineTraceForObjects (Transformation|GetWorldLocation _array_element) (- (Transformation|GetWorldLocation _array_element) "0.000000,0.000000,50.000000") (Utilities|Array|MakeArray "ObjectTypeQuery1") false 0 "None"))
    (if _returnvalue
      (Utilities|FlowControl|DoOnce false
        (:Completed
          (Variables|Default|SetIsDrop false)
          (Utilities|Time|ClearandInvalidateTimerbyHandle (Variables|Default|GetDropTimer))))))
  (if (not (Variables|Default|GetIsDrop))
    (for _array_element_2 (Components|GetChildrenComponents (Variables|Default|GetDefaultSceneRoot) false)
      (bind _returnvalue_2 (Game|SpawnActorfromClass "/Game/BluePrints/Block/BP_SingleBlock.BP_SingleBlock_C" (Math|Transform|MakeTransform (Transformation|GetWorldLocation _array_element_2) "0, 0, 0" "1.000000,1.000000,1.000000") "Undefined" "MultiplyWithRoot" 0 0))
      (Rendering|Material|SetMaterial (Variables|/Game/BluePrints/Block/BP_SingleBlock.BP_SingleBlock_C|GetStaticMesh _returnvalue_2) 0 (Rendering|Material|GetMaterial (Variables|Default|GetCube1) 0)))
    (Game|SpawnActorfromClass "BP_Block_C" (Math|Transform|MakeTransform (Math|Vector|MakeVector 0.0 0.0 (Math|Conversions|ToFloat(Integer) (* (Variables|Default|GetZLocation) 50))) "0, 0, 0" "1.000000,1.000000,1.000000") "Undefined" "MultiplyWithRoot" 0 0)
    (Actor|DestroyActor)))

(event Custom|AddLocation
  ;[0.15 0.15 0.15 0.5] Down Move
  (if (Variables|Default|GetIsSPush)
    (if (Variables|Default|GetIsDrop)
      (Transformation|AddActorWorldOffset "0.000000,0.000000,-50.000000"))))

(event Custom|Left
  ;[0.15 0.15 0.15 0.5] Left Move
  (if (Variables|Default|GetIsAPush)
    (Transformation|AddActorWorldOffset "0.000000,50.000000,0.000000")))

(event Input|EnhancedActionEvents|EnhancedInputActionIA_Rotation
  (params (ActionValue :type Boolean) (ElapsedSeconds :type Float%20%28double-precision%29) (TriggeredSeconds :type Float%20%28double-precision%29) (InputAction :type Input%20Action%20Object%20Reference :default "/Game/IA_Rotation.IA_Rotation")))

(event Input|EnhancedActionEvents|EnhancedInputActionIA_DownMove
  (params (ActionValue :type Boolean) (ElapsedSeconds :type Float%20%28double-precision%29) (TriggeredSeconds :type Float%20%28double-precision%29) (InputAction :type Input%20Action%20Object%20Reference :default "/Game/IA_DownMove.IA_DownMove"))
  ;[0.15 0.15 0.15 0.5] Down Move
  (:Started
    (Variables|Default|SetIsSPush true)
    (Transformation|AddActorWorldOffset "0.000000,0.000000,-50.000000")
    (bind _returnvalue (Utilities|Time|SetTimerbyEvent (delegate Custom|AddLocation) (Variables|Default|GetTime) true))
    (Variables|Default|SetSPushTimer _returnvalue))
  (:Completed
    (Variables|Default|SetIsSPush false)
    (Utilities|Time|ClearandInvalidateTimerbyHandle (Variables|Default|GetSPushTimer))))

(event Input|EnhancedActionEvents|EnhancedInputActionIA_LeftMove
  (params (ActionValue :type Boolean) (ElapsedSeconds :type Float%20%28double-precision%29) (TriggeredSeconds :type Float%20%28double-precision%29) (InputAction :type Input%20Action%20Object%20Reference :default "/Game/IA_LeftMove.IA_LeftMove"))
  ;[0.15 0.15 0.15 0.5] Left Move
  (:Started
    (Variables|Default|SetIsAPush true)
    (Transformation|AddActorWorldOffset "0.000000,50.000000,0.000000")
    (bind _returnvalue (Utilities|Time|SetTimerbyEvent (delegate Custom|Left) (Variables|Default|GetTime) true))
    (Variables|Default|SetAPushTimer _returnvalue))
  (:Completed
    (Variables|Default|SetIsAPush false)
    (Utilities|Time|ClearandInvalidateTimerbyHandle (Variables|Default|GetAPushTimer))))

(event Input|EnhancedActionEvents|EnhancedInputActionIA_RightMove
  (params (ActionValue :type Boolean) (ElapsedSeconds :type Float%20%28double-precision%29) (TriggeredSeconds :type Float%20%28double-precision%29) (InputAction :type Input%20Action%20Object%20Reference :default "/Game/IA_RightMove.IA_RightMove"))
  ;[0.15 0.15 0.15 0.5] Right Move
  (:Started
    (Variables|Default|SetIsDPush true)
    (Transformation|AddActorWorldOffset "0.000000,-50.000000,0.000000")
    (bind _returnvalue (Utilities|Time|SetTimerbyEvent (delegate Custom|Right) (Variables|Default|GetTime) true))
    (Variables|Default|SetDPushTimer _returnvalue))
  (:Completed
    (Variables|Default|SetIsDPush false)
    (Utilities|Time|ClearandInvalidateTimerbyHandle (Variables|Default|GetDPushTimer))))

(event EventBeginPlay
  (Utilities|FlowControl|Sequence
    (:then_0
      (bind _returnvalue (Actor|GetActorOfClass "/Script/Tetris.TetrisBoard"))
      (Utilities|FlowControl|Sequence
        (:then_0
          (bind _output_get (Variables|Default|SetZLocation (Variables|/Script/Tetris.TetrisBoard|GetBoardHeight _returnvalue)))
          (Transformation|SetActorLocation (Math|Vector|MakeVector 0.0 0.0 (Math|Conversions|ToFloat(Integer) (* _output_get 50))) false false))
        (:then_1
          (Variables|Default|SetYLocation (Variables|/Script/Tetris.TetrisBoard|GetBoardWidth _returnvalue)))))
    (:then_1
      (Variables|Default|SetTime 0.1)
      (bind _returnvalue_2 (Utilities|Time|SetTimerbyEvent (delegate Custom|DropBlock) (Variables|Default|GetTime) true))
      (Variables|Default|SetDropTimer _returnvalue_2))))

(event Collision|EventActorBeginOverlap
  (params (OtherActor :type Actor%20Object%20Reference)))

(event EventTick
  (params (DeltaSeconds :type Float%20%28single-precision%29)))

(fn ConstructionScript
  (switch int (Math|Random|RandomIntegerinRange 0 6)
    (:0
      ;[0.15 0.15 0.15 0.5] LineBlock
      (Transformation|AddLocalOffset (Variables|Default|GetCube2) "0.000000,0.000000,50.000000" false false)
      (Transformation|AddLocalOffset (Variables|Default|GetCube3) "0.000000,0.000000,100.000000" false false)
      (Transformation|AddLocalOffset (Variables|Default|GetCube4) "0.000000,0.000000,150.000000" false false)
      (Rendering|Material|SetMaterial (Variables|Default|GetCube1) 0 "/Game/Resource/M_SkyBlue.M_SkyBlue"))
    (:1
      ;[0.15 0.15 0.15 0.5] LBlock
      (Transformation|AddLocalOffset (Variables|Default|GetCube2) "0.000000,0.000000,50.000000" false false)
      (Transformation|AddLocalOffset (Variables|Default|GetCube3) "0.000000,0.000000,100.000000" false false)
      (Transformation|AddLocalOffset (Variables|Default|GetCube4) "0.000000,50.000000,0.000000" false false)
      (Rendering|Material|SetMaterial (Variables|Default|GetCube1) 0 "/Game/Resource/M_Blue.M_Blue"))
    (:2
      ;[0.15 0.15 0.15 0.5] Reverse L Block
      (Transformation|AddLocalOffset (Variables|Default|GetCube2) "0.000000,0.000000,50.000000" false false)
      (Transformation|AddLocalOffset (Variables|Default|GetCube3) "0.000000,0.000000,100.000000" false false)
      (Transformation|AddLocalOffset (Variables|Default|GetCube4) "0.000000,-50.000000,0.000000" false false)
      (Rendering|Material|SetMaterial (Variables|Default|GetCube1) 0 "/Game/Resource/M_Orange.M_Orange"))
    (:3
      ;[0.15 0.15 0.15 0.5] S Block
      (Transformation|AddLocalOffset (Variables|Default|GetCube2) "0.000000,0.000000,50.000000" false false)
      (Transformation|AddLocalOffset (Variables|Default|GetCube3) "0.000000,50.000000,50.000000" false false)
      (Transformation|AddLocalOffset (Variables|Default|GetCube4) "0.000000,50.000000,100.000000" false false)
      (Rendering|Material|SetMaterial (Variables|Default|GetCube1) 0 "/Game/Resource/M_YellowGreen.M_YellowGreen"))
    (:4
      ;[0.15 0.15 0.15 0.5] Reverse S Block
      (Transformation|AddLocalOffset (Variables|Default|GetCube2) "0.000000,0.000000,50.000000" false false)
      (Transformation|AddLocalOffset (Variables|Default|GetCube3) "0.000000,-50.000000,50.000000" false false)
      (Transformation|AddLocalOffset (Variables|Default|GetCube4) "0.000000,-50.000000,100.000000" false false)
      (Rendering|Material|SetMaterial (Variables|Default|GetCube1) 0 "/Game/Resource/M_Red.M_Red"))
    (:5
      ;[0.15 0.15 0.15 0.5] T Block
      (Transformation|AddLocalOffset (Variables|Default|GetCube2) "0.000000,0.000000,-50.000000" false false)
      (Transformation|AddLocalOffset (Variables|Default|GetCube3) "0.000000,50.000000,0.000000" false false)
      (Transformation|AddLocalOffset (Variables|Default|GetCube4) "0.000000,0.000000,50.000000" false false)
      (Rendering|Material|SetMaterial (Variables|Default|GetCube1) 0 "/Game/Resource/M_Purple.M_Purple"))
    (:6
      ;[0.15 0.15 0.15 0.5] Square Block
      (Transformation|AddLocalOffset (Variables|Default|GetCube2) "0.000000,0.000000,50.000000" false false)
      (Transformation|AddLocalOffset (Variables|Default|GetCube3) "0.000000,50.000000,0.000000" false false)
      (Transformation|AddLocalOffset (Variables|Default|GetCube4) "0.000000,50.000000,50.000000" false false)
      (Rendering|Material|SetMaterial (Variables|Default|GetCube1) 0 "/Game/Resource/M_Yellow.M_Yellow"))))